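; BP_BasePuzzleVers1 is a pushable puzzle block that moves in grid steps when its Box or Mesh is hit.
; The hit impulse becomes a grid vector, and the block eases there with audio if the movement check finds it clear.
; It then repeatedly moves down until blocked.
; Landing on a BP_HalfBlock shifts it 200 units along that block's forward direction, measured from the half block, if that path is clear.
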(event `self.Box.OnComponentHit`
  (params (HitComponent :type "PrimitiveComponent Object Reference") (OtherActor :type "Actor Object Reference") (OtherComp :type "PrimitiveComponent Object Reference") (NormalImpulse :type "Vector Structure") (Hit :type "HitResult Structure (by ref)"))
  (`self.OnHit` NormalImpulse))

(event `self.Mesh.OnComponentHit`
  (params (HitComponent :type "PrimitiveComponent Object Reference") (OtherActor :type "Actor Object Reference") (OtherComp :type "PrimitiveComponent Object Reference") (NormalImpulse :type "Vector Structure") (Hit :type "HitResult Structure (by ref)"))
  (`self.OnHit` NormalImpulse))

(event `OnHit`
  (params (Impulse :type "Vector Structure"))
  (bind _returnvalue (`self.K2_GetActorLocation`))
  (bind _box (`self.Box`))
  ;[1 1 1] Move Block on hit
  (bind _gridvector (`/Game/ShiftingHome/Library/ShiftingHomeFunctionLibrary.ImpulseToGridVector` Impulse))
  (bind _result (`/Game/ShiftingHome/Library/ShiftingHomeFunctionLibrary.IsVectorMovementBlocked` _returnvalue _gridvector self))
  (if (not _result)
    (`AddComponent|NODE_AddAudioComponent-2`)
    (`KismetSystemLibrary.MoveComponentTo` _box (+ _returnvalue _gridvector) (`SceneComponent.RelativeRotation` _box) true false 1.0)
    (`self.MoveBlockDownIfNotBlocked`)))

(event `MoveBlockDownIfNotBlocked`
  (bind _box (`self.Box`))
  ;[1 1 1] Move block down
  (bind _gridvector (`/Game/ShiftingHome/Library/ShiftingHomeFunctionLibrary.ImpulseToGridVector` (0.0 0.0 1.0)))
  (bind (_result _hitactor _targetlocation) (`/Game/ShiftingHome/Library/ShiftingHomeFunctionLibrary.IsVectorMovementBlocked` (`SceneComponent.K2_GetComponentLocation` (`self.Box`)) _gridvector self))
  (if _result
    (if (`self.Debug`)
      (`KismetSystemLibrary.PrintString` (`KismetStringLibrary.Concat_StrStr` "Blocked by " (`KismetSystemLibrary.GetDisplayName` _hitactor))))
    (`self.ProcessSpecialBlocks` _hitactor)
    (else
      (`AddComponent|NODE_AddAudioComponent-1`)
      (`KismetSystemLibrary.MoveComponentTo` _box _targetlocation (`SceneComponent.RelativeRotation` _box) true true 1.0)
      (`self.MoveBlockDownIfNotBlocked`))))

(event `ProcessSpecialBlocks`
  (params (BlockingActor :type "Actor Object Reference"))
  (bind _box (`self.Box`))
  ;[1 1 1] Process Special Blocks
  (bind _asbp_half_block (cast `/Game/ShiftingHome/LevelArchitecture/Static/BP_HalfBlock` BlockingActor))
  (bind (_result _hitactor _targetlocation) (`/Game/ShiftingHome/Library/ShiftingHomeFunctionLibrary.IsVectorMovementBlocked` (`self.K2_GetActorLocation` _asbp_half_block) (* (`KismetMathLibrary.Normal` (`self.GetActorForwardVector` _asbp_half_block)) 200.0) _asbp_half_block))
  (if _result
    (`KismetSystemLibrary.PrintString` (`KismetStringLibrary.Concat_StrStr` "Blocked by " (`KismetSystemLibrary.GetClassDisplayName` (`GameplayStatics.GetObjectClass` _hitactor))))
    (else
      (`AddComponent|NODE_AddAudioComponent-0`)
      (`KismetSystemLibrary.MoveComponentTo` _box _targetlocation (`SceneComponent.RelativeRotation` _box) true true 1.0))))

(fn `UserConstructionScript`
  (`parent.UserConstructionScript`))