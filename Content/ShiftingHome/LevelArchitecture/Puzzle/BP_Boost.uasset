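; BP_Boost is a puzzle boost actor that launches the player's ball when the character enters its trigger.
; On overlap it casts to ShiftingHomeCharacter and applies a mass-dependent impulse to the Ball along the Arrow's horizontal forward direction plus an upward component, scaled by BoostPower.
; Box and Mesh hit events forward their impulse to OnHit, which is empty despite its move-block comment.
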(event `self.Box.OnComponentHit`
  (params (HitComponent :type "PrimitiveComponent Object Reference") (OtherActor :type "Actor Object Reference") (OtherComp :type "PrimitiveComponent Object Reference") (NormalImpulse :type "Vector Structure") (Hit :type "HitResult Structure (by ref)"))
  (`self.OnHit` NormalImpulse))

(event `self.Mesh.OnComponentHit`
  (params (HitComponent :type "PrimitiveComponent Object Reference") (OtherActor :type "Actor Object Reference") (OtherComp :type "PrimitiveComponent Object Reference") (NormalImpulse :type "Vector Structure") (Hit :type "HitResult Structure (by ref)"))
  (`self.OnHit` NormalImpulse))

(event `OnHit`
  (params (Impulse :type "Vector Structure"))
  ;[1 1 1] Move Block on hit
)

(event `self.Trigger.OnComponentBeginOverlap`
  (params (OverlappedComponent :type "PrimitiveComponent Object Reference") (OtherActor :type "Actor Object Reference") (OtherComp :type "PrimitiveComponent Object Reference") (OtherBodyIndex :type Integer) (bFromSweep :type Boolean) (SweepResult :type "HitResult Structure (by ref)"))
  (bind (_returnvalue_x _returnvalue_y) (`KismetMathLibrary.BreakVector` (`SceneComponent.GetForwardVector` (`self.Arrow`))))
  (bind _asshifting_home_character (cast `/Game/ShiftingHome/Player/ShiftingHomeCharacter` OtherActor))
  (`PrimitiveComponent.AddImpulse` (`/Game/ShiftingHome/Player/ShiftingHomeCharacter.Ball` _asshifting_home_character) (* (`KismetMathLibrary.MakeVector` _returnvalue_x _returnvalue_y 1.0) (`self.BoostPower`)) "None" false))

(fn `UserConstructionScript`
  (`parent.UserConstructionScript`))