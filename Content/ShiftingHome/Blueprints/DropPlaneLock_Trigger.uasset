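; Trigger actor that catches a BP_FloatingBlock on overlap, locks it to a plane and lowers it.
; The block snaps to the trigger's position offset along negative Y, then its Box gets a YZ-plane constraint and has physics simulation turned off.
; MoveComponentTo then eases the Box downward over a few seconds, targeting a point below the block's new location while keeping its rotation.
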(event `self.ReceiveActorBeginOverlap`
  (params (OtherActor :type "Actor Object Reference"))
  (bind (_returnvalue_x _returnvalue_y _returnvalue_z) (`KismetMathLibrary.BreakVector` (`self.K2_GetActorLocation` self)))
  (bind _asbp_floating_block (cast `/Game/ShiftingHome/LevelArchitecture/BP_FloatingBlock` OtherActor))
  (`self.K2_SetActorLocation` _asbp_floating_block (`KismetMathLibrary.MakeVector` _returnvalue_x (- _returnvalue_y 200.0) _returnvalue_z) false false)
  (bind _box (`/Game/ShiftingHome/LevelArchitecture/BP_BaseBlock.Box` _asbp_floating_block))
  (`PrimitiveComponent.SetConstraintMode` _box "YZPlane")
  (`PrimitiveComponent.SetSimulatePhysics` _box false)
  (`KismetSystemLibrary.MoveComponentTo` _box (+ (`self.K2_GetActorLocation` _asbp_floating_block) (`KismetMathLibrary.MakeVector` 0.0 0.0 -200.0)) (`self.K2_GetActorRotation` _asbp_floating_block) true false 3.0))

(fn `UserConstructionScript`)