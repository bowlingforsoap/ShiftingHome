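; BlockSpawner is an actor that periodically spawns instances of a configurable class at random horizontal positions around itself.
; A looping timer started on BeginPlay fires every SpawnRate seconds to spawn one SpawnClass actor using the spawner's rotation.
; X and Y are randomly offset within plus or minus SpawnRadius, while Z is set to negative SpawnRadius in world space, ignoring the spawner's height.
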(event `self.ReceiveBeginPlay`
  (`KismetSystemLibrary.K2_SetTimerDelegate` (delegate `CustomEvent_0`) (`self.SpawnRate`) true))

(event `CustomEvent_0`
  (bind (_returnvalue_x _returnvalue_y) (`KismetMathLibrary.BreakVector` (`self.K2_GetActorLocation`)))
  (bind _spawnradius (`self.SpawnRadius`))
  (bind _returnvalue (* _spawnradius -1.0))
  (`|SpawnActorFromClass` (`self.SpawnClass`) (`KismetMathLibrary.MakeTransform` (`KismetMathLibrary.MakeVector` (+ _returnvalue_x (`KismetMathLibrary.RandomFloatInRange` _returnvalue _spawnradius)) (+ _returnvalue_y (`KismetMathLibrary.RandomFloatInRange` _returnvalue _spawnradius)) _returnvalue) (`self.K2_GetActorRotation`)) "Undefined" "OverrideRootScale" null null))

(fn `UserConstructionScript`)